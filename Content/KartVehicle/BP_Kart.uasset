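; Player kart pawn driven by Enhanced Input, with steering, drifting, jumping, fuel-gated boost and respawn at the GameState's current checkpoint.
; Tick line-traces five suspension points, applying spring and drive forces to a physics Box at each.
; Steering applies yaw torque, while shifting center of mass shapes acceleration, turning and jumping.
; Ground checks switch between clamped ground rotation and extra downforce with air leveling; drifting yaws a pivot and sets a speed multiplier.
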(event OnComponentBeginOverlap(Anti_Collision)
  (params (OverlappedComponent :type Primitive%20Component%20Object%20Reference) (OtherActor :type Actor%20Object%20Reference) (OtherComp :type Primitive%20Component%20Object%20Reference) (OtherBodyIndex :type Integer) (bFromSweep :type Boolean) (SweepResult :type Hit%20Result%20Structure%20%28by%20ref%29)))

(event Input|EnhancedActionEvents|EnhancedInputActionIA_Acceleration
  (params (ActionValue :type Float%20%28double-precision%29) (ElapsedSeconds :type Float%20%28double-precision%29) (TriggeredSeconds :type Float%20%28double-precision%29) (InputAction :type Input%20Action%20Object%20Reference :default "/Game/Blueprints/Inputs/IA_Acceleration.IA_Acceleration"))
  (bind _output_get (Variables|Default|SetAccelerationInput (Math|Interpolation|FInterpTo (Variables|Default|GetAccelerationInput) (Math|Float|SelectFloat ActionValue 0.5 (CallFunction|IsGrounded)) (Utilities|Time|GetWorldDeltaSeconds) 1.75)))
  (Development|PrintString (Utilities|String|ToString(Float) _output_get)))

(event Input|EnhancedActionEvents|EnhancedInputActionIA_Steer
  (params (ActionValue :type Float%20%28double-precision%29) (ElapsedSeconds :type Float%20%28double-precision%29) (TriggeredSeconds :type Float%20%28double-precision%29) (InputAction :type Input%20Action%20Object%20Reference :default "/Game/Blueprints/Inputs/IA_Steer.IA_Steer"))
  (CallFunction|TurnKart ActionValue ActionValue 0.0))

(event Input|EnhancedActionEvents|EnhancedInputActionIA_Boost
  (params (ActionValue :type Boolean) (ElapsedSeconds :type Float%20%28double-precision%29) (TriggeredSeconds :type Float%20%28double-precision%29) (InputAction :type Input%20Action%20Object%20Reference :default "/Game/Blueprints/Inputs/IA_Boost.IA_Boost"))
  (:Started
    (if (> (Variables|/Game/Blueprints/GS_GameState.GS_GameState_C|GetFuel (.AsGS%20Game%20State (Utilities|Casting|CastToGS_GameState (Game|GetGameState)))) 0.0)
      (CallFunction|BoostKart 2.0)))
  (:Completed
    (CallFunction|ResetBoost 1.0)))

(event Input|EnhancedActionEvents|EnhancedInputActionIA_Drift
  (params (ActionValue :type Boolean) (ElapsedSeconds :type Float%20%28double-precision%29) (TriggeredSeconds :type Float%20%28double-precision%29) (InputAction :type Input%20Action%20Object%20Reference :default "/Game/Blueprints/Inputs/IA_Drift.IA_Drift"))
  (:Started
    (CallFunction|StartDrift))
  (:Canceled
    (CallFunction|StopDrift :!label _label))
  (:Completed
    (goto _label)))

(event Input|EnhancedActionEvents|EnhancedInputActionIA_Jump
  (params (ActionValue :type Boolean) (ElapsedSeconds :type Float%20%28double-precision%29) (TriggeredSeconds :type Float%20%28double-precision%29) (InputAction :type Input%20Action%20Object%20Reference :default "/Game/Blueprints/Inputs/IA_Jump.IA_Jump"))
  (if (CallFunction|IsGrounded)
    (CallFunction|Jump)))

(event EventBeginPlay
  (Input|AddMappingContext (PlayerController|LocalPlayerSubsystems|GetEnhancedInputLocalPlayerSubsystem (Game|GetPlayerController 0)) "/Game/Blueprints/Inputs/IMC_Vehicle.IMC_Vehicle" 0 "(bIgnoreAllPressedKeysUntilRelease=True,bForceImmediately=False,bNotifyUserSettings=False)")
  (bind _outactors (Actor|GetAllActorsOfClass "/Game/Blueprints/BP_CheckPoint.BP_CheckPoint_C"))
  (Variables|Default|SetStoredCheckpoitns _outactors))

(event Collision|EventActorBeginOverlap
  (params (OtherActor :type Actor%20Object%20Reference)))

(event EventTick
  (params (DeltaSeconds :type Float%20%28single-precision%29))
  (CallFunction|Suspension (Variables|Default|GetHead))
  (CallFunction|Suspension (Variables|Default|GetWL_Wing))
  (CallFunction|Suspension (Variables|Default|GetWR_Wing))
  (CallFunction|Suspension (Variables|Default|GetBL_Jet))
  (CallFunction|Suspension (Variables|Default|GetBR_Jet))
  (if (CallFunction|IsGrounded)
    (CallFunction|CalculateAcceleration)
    (CallFunction|LimitGroundRotation)
    (if (== (Variables|/Game/Blueprints/GS_GameState.GS_GameState_C|GetFuel (.AsGS%20Game%20State (Utilities|Casting|CastToGS_GameState (Game|GetGameState)))) 0.0)
      (CallFunction|ResetBoost 1.0))
    (else
      (Physics|AddForce (Variables|Default|GetBox) (Math|Vector|SelectVector "0, 0, 0" "0.000000,0.000000,-2500.000000" (CallFunction|IsGrounded)) "None" false)
      (CallFunction|SetAirRotations))))

(event Input|KeyboardEvents|F
  (params (Key :type Key%20Structure :default "None"))
  (:Pressed
    (CallFunction|RespawnatCheckpoint)))

(fn ConstructionScript)

(fn Suspension
  (params (Suspension%20points :type Scene%20Component%20Object%20Reference))
  (bind _returnvalue (Transformation|GetWorldLocation Suspension%20points))
  (bind _outhit (Collision|LineTraceByChannel _returnvalue (+ _returnvalue (* (Math|Vector|GetUpVector Suspension%20points) -8e+01)) "TraceTypeQuery1" false 0 "ForOneFrame"))
  (if (.bBlockingHit (Collision|BreakHitResult _outhit))
    (Class|PrimitiveComponent|AddForceatLocation (Variables|Default|GetBox) (* (- 1.0 (Math|Float|NormalizetoRange (.Distance (Collision|BreakHitResult _outhit)) 0.0 8e+01)) (Math|Vector|GetUnitDirection(Vector) (.TraceEnd (Collision|BreakHitResult _outhit)) (.TraceStart (Collision|BreakHitResult _outhit))) 1.5e+06) (Transformation|GetWorldLocation Suspension%20points) "None")
    (CallFunction|AccelerateKart Suspension%20points)
    (else
      (CallFunction|AccelerateKart Suspension%20points)
      (CallFunction|TurnKart 0.0 0.0 0.0))))

(fn CalculateAcceleration
  (bind _pivotpoint (Variables|Default|GetPivotPoint))
  (Variables|Default|SetAcceleration (* (Math|Float|Lerp 0.0 (Variables|Default|GetMaxAcceleration) (Variables|Default|GetAccelerationInput)) (Variables|Default|GetAccelerationInput)))
  (Variables|Default|SetAccelerationInput (Math|Interpolation|FInterpTo (Variables|Default|GetAccelerationInput) 0.0 (Utilities|Time|GetWorldDeltaSeconds) 1.0))
  (Transformation|SetRelativeRotation _pivotpoint (Math|Rotator|MakeRotator 0.0 0.0 (.yaw (Math|Interpolation|RInterpTo (Variables|/Script/Engine.SceneComponent|GetRelativeRotation _pivotpoint) (Variables|Default|GetDriftRotation) (Utilities|Time|GetWorldDeltaSeconds) (Math|Float|SelectFloat 0.5 4.0 (Variables|Default|GetisDrifting))))) false false))

(fn AccelerateKart
  (params (Suspension%20Points :type Scene%20Component%20Object%20Reference))
  (bind _speedmodifer (Variables|Default|GetSpeedModifer))
  (bind _driftboostmod (Variables|Default|GetDriftBoostMod))
  (bind _roadmodifier (Variables|Default|GetRoadModifier))
  (bind _box (Variables|Default|GetBox))
  (bind _accelerationinput (Variables|Default|GetAccelerationInput))
  (bind _returnvalue (Math|Vector|GetForwardVector _box))
  (bind _returnvalue_2 (Physics|GetMass _box))
  (bind _returnvalue_3 (* _returnvalue 2e+03 _accelerationinput _returnvalue_2 _speedmodifer _driftboostmod _roadmodifier))
  (Class|PrimitiveComponent|AddForceatLocation (Variables|Default|GetBox) (Math|Vector|SelectVector (/ _returnvalue_3 "2.000000,2.000000,1.000000") _returnvalue_3 (== (Variables|/Game/Blueprints/GS_GameState.GS_GameState_C|GetFuel (.AsGS%20Game%20State (Utilities|Casting|CastToGS_GameState (Game|GetGameState)))) 0.0)) (Transformation|GetWorldLocation Suspension%20Points) "None")
  (Class|PrimitiveComponent|SetCenterOfMass (Variables|Default|GetBox) (* "50.000000,0.000000,0.000000" (Variables|Default|GetAccelerationInput)) "None"))

(fn IsGrounded
  (bind _box (Variables|Default|GetBox))
  (bind _returnvalue (Transformation|GetWorldLocation _box))
  (bind _returnvalue_2 (Collision|LineTraceByChannel _returnvalue (- _returnvalue "0.000000,0.000000,100.000000") "TraceTypeQuery1" false 0 "ForOneFrame"))
  (return _returnvalue_2))

(fn TurnKart
  (params (Target :type Float%20%28double-precision%29) (InputPin :type Float%20%28double-precision%29) (DriftSteer :type Float%20%28double-precision%29))
  (if (Variables|Default|GetIsBoosting)
    (Variables|Default|SetsteeringMulti (* (Variables|Default|GetMaxSteeringMulti) 0.75))
    (Variables|Default|SetCurrentTurningTorque (* (Variables|Default|GetMaxTurnTorque) 0.75))
    (else
      (Variables|Default|SetsteeringMulti (Variables|Default|GetMaxSteeringMulti))
      (Variables|Default|SetCurrentTurningTorque (Variables|Default|GetMaxTurnTorque))))
  (bind _output_get (Variables|Default|SetDriftSteer (Math|Float|Clamp(Float) (Math|Float|SelectFloat (* (Math|Float|Max(Float) (Variables|Default|GetDriftSteer) (Math|Float|Absolute(Float) InputPin)) (Math|Float|Sign(Float) (.yaw (Variables|Default|GetDriftRotation)))) InputPin (Variables|Default|GetisDrifting)) -3.0 3.0)))
  (Variables|Default|SetTurnInput (Math|Interpolation|FInterpTo (Variables|Default|GetTurnInput) Target (Utilities|Time|GetWorldDeltaSeconds) 0.5))
  (Class|PrimitiveComponent|AddTorqueinRadians (Variables|Default|GetBox) (Math|Vector|MakeVector 0.0 0.0 (* _output_get (Variables|Default|GetCurrentTurningTorque) (Variables|Default|GetsteeringMulti))) "None" false)
  (if (> (* (Variables|Default|GetTurnInput) 1.0) 0.1)
    (Class|PrimitiveComponent|SetCenterOfMass (Variables|Default|GetBox) (* "0.000000,50.000000,0.000000" (Math|Interpolation|FInterpTo (Math|Conversions|ToFloat(Integer) (Utilities|String|ToString(Integer) (Physics|GetCenterOfMass (Variables|Default|GetBox) "None"))) 15.0 (Utilities|Time|GetWorldDeltaSeconds) (Variables|Default|GetCenterOfMassSpeed))) "None")
    (elif (< (* (Variables|Default|GetTurnInput) -1.0) -0.1)
      (Class|PrimitiveComponent|SetCenterOfMass (Variables|Default|GetBox) (* "0.000000,-50.000000,0.000000" (Math|Interpolation|FInterpTo (Math|Conversions|ToFloat(Integer) (Utilities|String|ToString(Integer) (Physics|GetCenterOfMass (Variables|Default|GetBox) "None"))) 15.0 (Utilities|Time|GetWorldDeltaSeconds) (Variables|Default|GetCenterOfMassSpeed))) "None")
      (else
        (Class|PrimitiveComponent|SetCenterOfMass (Variables|Default|GetBox) "0, 0, 0" "None")))))

(fn BoostKart
  (params (SpeedModifer :type Float%20%28single-precision%29))
  (if (> (Variables|/Game/Blueprints/GS_GameState.GS_GameState_C|GetFuel (.AsGS%20Game%20State (Utilities|Casting|CastToGS_GameState (Game|GetGameState)))) 0.0)
    (Variables|Default|SetSpeedModifer SpeedModifer)
    (Variables|Default|SetCanDrift false)
    (Variables|/Game/Blueprints/GS_GameState.GS_GameState_C|SetIsBoosting (.AsGS%20Game%20State (Utilities|Casting|CastToGS_GameState (Game|GetGameState))) true)
    (Variables|Default|SetIsBoosting true)
    (else
      (CallFunction|ResetBoost 1.0))))

(fn ResetBoost
  (params (SpeedModifer :type Float%20%28single-precision%29))
  (Variables|Default|SetSpeedModifer SpeedModifer)
  (Variables|Default|SetCanDrift true)
  (Variables|/Game/Blueprints/GS_GameState.GS_GameState_C|SetIsBoosting (.AsGS%20Game%20State (Utilities|Casting|CastToGS_GameState (Game|GetGameState))) false)
  (Variables|Default|SetIsBoosting false))

(fn StartDrift
  (Variables|Default|SetsteeringMulti (* (Variables|Default|GetMaxSteeringMulti) (Variables|Default|GetDriftMultiplier)))
  (Variables|Default|SetisDrifting true)
  (Variables|Default|SetDriftRotation (Math|Rotator|MakeRotator 0.0 0.0 (* (Math|Float|Sign(Float) (Input|EnhancedActionValues|GetIA_Steer)) 4e+01)))
  (CallFunction|DriftBoost (+ (/ (Math|Float|Absolute(Float) (Variables|Default|GetDriftSteer)) 3.0) 1.0)))

(fn StopDrift
  (Variables|Default|SetsteeringMulti (Variables|Default|GetMaxSteeringMulti))
  (Variables|Default|SetisDrifting false)
  (Variables|Default|SetDriftRotation "0, 0, 0"))

(fn RespawnatCheckpoint
  (bind _array_element (Utilities|Array|ForEachLoopwithBreak (Variables|Default|GetStoredCheckpoitns) :!label _label)
    (:LoopBody
      (if (== (Variables|/Game/Blueprints/BP_CheckPoint.BP_CheckPoint_C|GetCheckPoint _array_element) (Variables|/Game/Blueprints/GS_GameState.GS_GameState_C|GetCurrentCheckPoint (.AsGS%20Game%20State (Utilities|Casting|CastToGS_GameState (Game|GetGameState)))))
        (Default|RespawnPlayer _array_element)
        (goto _label Break)))
    (:Completed
      (Development|PrintString "No Checkpoint is valid"))))

(fn Jump
  (bind _box (Variables|Default|GetBox))
  (Class|PrimitiveComponent|SetCenterOfMass (Variables|Default|GetBox) "-20.000000,0.000000,0.000000" "None")
  (Class|PrimitiveComponent|AddForceatLocation _box "0.000000,0.000000,35000000.000000" (Variables|/Script/Engine.SceneComponent|GetRelativeLocation _box) "None")
  (CallFunction|SetAirRotations)
  (Class|PrimitiveComponent|SetCenterOfMass (Variables|Default|GetBox) (* "80.000000,0.000000,0.000000" (Math|Interpolation|FInterpTo -2e+01 8e+01 (Utilities|Time|GetWorldDeltaSeconds) 2e+01)) "None"))

(fn SetAirRotations
  (bind _returnvalue (Utilities|Time|GetWorldDeltaSeconds))
  (bind _box (Variables|Default|GetBox))
  (bind _relativerotation (Variables|/Script/Engine.SceneComponent|GetRelativeRotation _box))
  (bind _returnvalue_2 (Math|Float|Clamp(Float) (.pitch _relativerotation) -3e+01 3e+01))
  (bind _returnvalue_3 (Math|Interpolation|FInterpTo (.pitch _relativerotation) _returnvalue_2 _returnvalue 1e+01))
  (Transformation|SetRelativeRotation _box (Math|Rotator|MakeRotator (Math|Interpolation|FInterpTo (.roll _relativerotation) (Math|Float|Clamp(Float) (.roll _relativerotation) -3e+01 3e+01) _returnvalue 1e+01) _returnvalue_3 (.yaw _relativerotation)) false false)
  (Class|PrimitiveComponent|SetCenterOfMass (Variables|Default|GetBox) "15.000000,0.000000,0.000000" "None")
  (Transformation|SetRelativeRotation (Variables|Default|GetBox) (Math|Rotator|MakeRotator 0.0 (Math|Interpolation|FInterpTo _returnvalue_3 (Math|Float|Clamp(Float) _returnvalue_3 -5.0 5.0) (Utilities|Time|GetWorldDeltaSeconds) 1e+01) (.yaw _relativerotation)) false false))

(fn LimitGroundRotation
  (bind _box (Variables|Default|GetBox))
  (bind _relativerotation (Variables|/Script/Engine.SceneComponent|GetRelativeRotation _box))
  (Transformation|SetRelativeRotation _box (Math|Rotator|MakeRotator (Math|Interpolation|FInterpTo (.roll _relativerotation) (Math|Float|Clamp(Float) (.roll _relativerotation) -3e+01 3e+01) (Utilities|Time|GetWorldDeltaSeconds) 0.0) (Math|Interpolation|FInterpTo (.pitch _relativerotation) (Math|Float|Clamp(Float) (.pitch _relativerotation) -3e+01 3e+01) (Utilities|Time|GetWorldDeltaSeconds) 3e+01) (.yaw _relativerotation)) false false))

(fn DriftBoost
  (params (BoostModifier :type Float%20%28double-precision%29))
  (Variables|Default|SetDriftBoostMod BoostModifier))

(fn ResetDriftBoost
  (params (BoostModifier :type Float%20%28double-precision%29))
  (Variables|Default|SetDriftBoostMod BoostModifier))