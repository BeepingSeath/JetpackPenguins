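; BP_OilBomb is an oil drum hazard that explodes when its box is overlapped.
; The overlap passes FuelReduction to the game state's AddFuel, spawns explosion effects and destroys the actor.
; It also zeroes player 0 kart's acceleration and velocity around a backward-and-up impulse, without checking what overlapped.
; A timed hide-and-reappear respawn event exists, but its only call never runs.
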(event OnComponentBeginOverlap(Box)
  (params (OverlappedComponent :type Primitive%20Component%20Object%20Reference) (OtherActor :type Actor%20Object%20Reference) (OtherComp :type Primitive%20Component%20Object%20Reference) (OtherBodyIndex :type Integer) (bFromSweep :type Boolean) (SweepResult :type Hit%20Result%20Structure%20%28by%20ref%29))
  (bind _returnvalue (Game|Player|GetPlayerPawn 0))
  (bind _asbp_kart (Utilities|Casting|CastToBP_Kart _returnvalue))
  (bind _box (Variables|/Game/KartVehicle/BP_Kart.BP_Kart_C|GetBox _asbp_kart))
  (bind _returnvalue_2 (Math|Vector|GetForwardVector _box))
  (bind _returnvalue_3 (* _returnvalue_2 "-2000.000000,-2000.000000,0.000000"))
  (Default|AddFuel (.AsGS%20Game%20State (Utilities|Casting|CastToGS_GameState (Game|GetGameState))) (Variables|Default|GetFuelReduction))
  (Effects|SpawnEmitteratLocation "/Game/StarterContent/Particles/P_Explosion.P_Explosion" (Transformation|GetWorldLocation (Variables|Default|GetOilDrum)) "0, 0, 0" "5.000000,5.000000,5.000000")
  (Audio|SpawnSoundatLocation "/Game/Audio/explosion-312361.explosion-312361" "0, 0, 0" "0, 0, 0" 1.0 1.0 0.0 0 0)
  (Variables|/Game/KartVehicle/BP_Kart.BP_Kart_C|SetAccelerationInput _asbp_kart 0.0)
  (Physics|SetPhysicsLinearVelocity _box "0, 0, 0" false "None")
  (Physics|AddImpulse _box (Math|Vector|MakeVector (.x _returnvalue_3) (.y _returnvalue_3) 2e+03) "None" true)
  (Physics|SetPhysicsLinearVelocity _box "0, 0, 0" false "None")
  (Variables|/Game/KartVehicle/BP_Kart.BP_Kart_C|SetAccelerationInput _asbp_kart 0.0)
  (Actor|DestroyActor))

(event Custom|Hide%20&%20Reappear
  (bind _self self)
  (bind _defaultsceneroot (Variables|Default|GetDefaultSceneRoot _self))
  (Rendering|SetVisibility _defaultsceneroot false true)
  (Collision|SetActorEnableCollision false)
  (Utilities|FlowControl|Delay (Variables|Default|GetRespawnTimer))
  (Rendering|SetVisibility _defaultsceneroot true true)
  (Collision|SetActorEnableCollision true))

(event EventBeginPlay)

(event Collision|EventActorBeginOverlap
  (params (OtherActor :type Actor%20Object%20Reference)))

(event EventTick
  (params (DeltaSeconds :type Float%20%28single-precision%29)))

(fn ConstructionScript)