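; BP_Door is a key-locked sliding door that opens when something enters its KeyCheck trigger while the game state's HasKey flag is set.
; BeginPlay caches the Cube's origin and its full X width as the slide offset.
; The Opening timeline lerps the Cube sideways along local X by that width via DoorMovement, then reverses to close it after a Duration delay.
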(event OnComponentBeginOverlap(KeyCheck)
  (params (OverlappedComponent :type Primitive%20Component%20Object%20Reference) (OtherActor :type Actor%20Object%20Reference) (OtherComp :type Primitive%20Component%20Object%20Reference) (OtherBodyIndex :type Integer) (bFromSweep :type Boolean) (SweepResult :type Hit%20Result%20Structure%20%28by%20ref%29))
  (if (Variables|/Game/Blueprints/GS_GameState.GS_GameState_C|GetHasKey (.AsGS%20Game%20State (Utilities|Casting|CastToGS_GameState (Game|GetGameState))))
    (CallFunction|OpenDoor)
    (Utilities|FlowControl|Delay (Variables|Default|GetDuration))
    (CallFunction|CloseDoor)))

(event Custom|CloseDoor
  (bind _dooranimation (Timeline|Opening Reverse)
    (:Update
      (CallFunction|DoorMovement (Variables|Default|GetOffsetX) _dooranimation))))

(event Custom|OpenDoor
  (bind _dooranimation (Timeline|Opening Play)
    (:Update
      (CallFunction|DoorMovement (Variables|Default|GetOffsetX) _dooranimation))))

(event EventBeginPlay
  (Variables|Default|SetDoorOrigin (Variables|/Script/Engine.SceneComponent|GetRelativeLocation (Variables|Default|GetCube)))
  (Variables|Default|SetOffsetX (* (.x (.BoxExtent (Collision|GetComponentBounds (Variables|Default|GetCube)))) 2.0)))

(event Collision|EventActorBeginOverlap
  (params (OtherActor :type Actor%20Object%20Reference)))

(event EventTick
  (params (DeltaSeconds :type Float%20%28single-precision%29)))

(fn ConstructionScript)

(fn DoorMovement
  (params (OffsetX :type Float%20%28double-precision%29) (Alpha :type Float%20%28single-precision%29))
  (bind _doororigin (Variables|Default|GetDoorOrigin))
  (bind (_x _y _z) (Math|Vector|BreakVector _doororigin))
  (Transformation|SetRelativeLocation (Variables|Default|GetCube) (Math|Vector|Lerp(Vector) (Variables|Default|GetDoorOrigin) (Math|Vector|MakeVector (+ OffsetX _x) _y _z) Alpha) false false))