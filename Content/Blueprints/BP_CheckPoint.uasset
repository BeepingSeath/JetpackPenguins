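; Race checkpoint for the kart game that enforces track order, with checkpoint 0 acting as the finish line.
; Box overlaps advance GS_GameState's current checkpoint only in sequence, without filtering the overlapping actor.
; The finish line requires the last checkpoint, then resets progress, counts the lap and either finalizes the race or sets best lap time.
; RespawnPlayer moves the first BP_Kart found to the box, offsetting its Box yaw by 90 degrees.
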(event OnComponentBeginOverlap(Box)
  (params (OverlappedComponent :type Primitive%20Component%20Object%20Reference) (OtherActor :type Actor%20Object%20Reference) (OtherComp :type Primitive%20Component%20Object%20Reference) (OtherBodyIndex :type Integer) (bFromSweep :type Boolean) (SweepResult :type Hit%20Result%20Structure%20%28by%20ref%29))
  (bind _returnvalue (Game|GetGameState))
  (bind _asgs_game_state (Utilities|Casting|CastToGS_GameState _returnvalue))
  (if (!= (Variables|Default|GetCheckPoint) 0)
    (if (== (- (Variables|Default|GetCheckPoint) 1) (Variables|/Game/Blueprints/GS_GameState.GS_GameState_C|GetCurrentCheckPoint _asgs_game_state))
      (Variables|/Game/Blueprints/GS_GameState.GS_GameState_C|SetCurrentCheckpoint _asgs_game_state (Variables|Default|GetCheckPoint)))
    (else
      (CallFunction|FinishLine))))

(event Custom|RespawnPlayer
  (bind _returnvalue (Actor|GetActorOfClass "/Game/KartVehicle/BP_Kart.BP_Kart_C"))
  (CallFunction|Respawn _returnvalue))

(event Custom|FinishLine
  (bind _returnvalue (Game|GetGameState))
  (bind _asgs_game_state (Utilities|Casting|CastToGS_GameState _returnvalue))
  (if (== (Variables|/Game/Blueprints/GS_GameState.GS_GameState_C|GetCurrentCheckPoint _asgs_game_state) (Variables|Default|GetMaxCheckPoint))
    (Variables|/Game/Blueprints/GS_GameState.GS_GameState_C|SetCurrentCheckPoint _asgs_game_state (Variables|Default|GetCheckPoint))
    (bind _result (Math|Integer|IncrementInt (Variables|/Game/Blueprints/GS_GameState.GS_GameState_C|GetLaps _asgs_game_state))
      (:%20%20
        (if (== _result (Variables|Default|GetMaxLaps))
          (Default|FinalizeRace _asgs_game_state)
          (else
            (Default|SetBestLapTime _asgs_game_state)))))))

(event EventBeginPlay)

(event Collision|EventActorBeginOverlap
  (params (OtherActor :type Actor%20Object%20Reference)))

(event EventTick
  (params (DeltaSeconds :type Float%20%28single-precision%29)))

(fn ConstructionScript)

(fn Respawn
  (params (self2 :type BP%20Kart%20Object%20Reference))
  (bind _box (Variables|Default|GetBox))
  (bind _box_2 (Variables|Default|GetBox))
  (bind _returnvalue (Transformation|GetWorldRotation _box))
  (bind _returnvalue_2 (Transformation|SetActorLocationAndRotation self2 (Transformation|GetWorldLocation _box_2) (Transformation|GetWorldRotation _box_2)))
  (Development|PrintString (Utilities|String|ToString(Boolean) _returnvalue_2))
  (Transformation|SetWorldLocationAndRotation (Variables|/Game/KartVehicle/BP_Kart.BP_Kart_C|GetBox self2) (Transformation|GetWorldLocation _box) (Math|Rotator|MakeRotator (.roll _returnvalue) (.pitch _returnvalue) (+ 9e+01 (.yaw _returnvalue))) false false))