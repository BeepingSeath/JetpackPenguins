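; BP_FuelPickup is a respawning pickup that adds fuel through the game state.
; Any overlap with its Box calls AddFuel on GS_GameState with its Amount, without checking the overlapping actor.
; It then plays a pickup sound at the Box's relative location, rather than its world location.
; The actor then hides and disables collision, restoring both after a RespawnTime delay instead of being destroyed.
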(event OnComponentBeginOverlap(Box)
  (params (OverlappedComponent :type Primitive%20Component%20Object%20Reference) (OtherActor :type Actor%20Object%20Reference) (OtherComp :type Primitive%20Component%20Object%20Reference) (OtherBodyIndex :type Integer) (bFromSweep :type Boolean) (SweepResult :type Hit%20Result%20Structure%20%28by%20ref%29))
  (Default|AddFuel (.AsGS%20Game%20State (Utilities|Casting|CastToGS_GameState (Game|GetGameState))) (Variables|Default|GetAmount))
  (Audio|SpawnSoundatLocation "/Game/Audio/pick-up-sfx-38516.pick-up-sfx-38516" (Variables|/Script/Engine.SceneComponent|GetRelativeLocation (Variables|Default|GetBox)) "0, 0, 0" 1.0 1.0 0.0 0 0)
  (CallFunction|Hide&Reappear))

(event Custom|Hide%20&%20Reappear
  (bind _self self)
  (bind _defaultsceneroot (Variables|Default|GetDefaultSceneRoot _self))
  (Rendering|SetVisibility _defaultsceneroot false true)
  (Collision|SetActorEnableCollision false)
  (Utilities|FlowControl|Delay (Variables|Default|GetRespawnTime))
  (Rendering|SetVisibility _defaultsceneroot true true)
  (Collision|SetActorEnableCollision true))

(event EventBeginPlay)

(event Collision|EventActorBeginOverlap
  (params (OtherActor :type Actor%20Object%20Reference)))

(event EventTick
  (params (DeltaSeconds :type Float%20%28single-precision%29)))

(fn ConstructionScript)