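; Game state for a kart race that tracks fuel, total and lap times, and the best lap.
; Until the race finishes, Tick advances both timers and drains fuel by BP_Kart's absolute acceleration input, scaled while boosting by boost cost and the player kart's speed modifier.
; AddFuel refills up to the maximum, and SetBestLapTime records improved laps and resets the lap timer.
; FinalizeRace stops updates, records the last lap and prints the results.
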(event Custom|AddFuel
  (params (Amount :type Float%20%28double-precision%29))
  (bind _output_get (Variables|Default|SetFuel (+ Amount (Variables|Default|GetFuel))))
  (if (> _output_get (Variables|Default|GetMaxFuel))
    (Variables|Default|SetFuel (Variables|Default|GetMaxFuel)))
  (Development|PrintText (Utilities|Text|ToText(Float) (Variables|Default|GetFuel) "HalfToEven")))

(event Custom|DecreaseFuel
  (params (DeltaTime :type Float%20%28double-precision%29))
  (bind _returnvalue (Actor|GetActorOfClass "/Game/KartVehicle/BP_Kart.BP_Kart_C"))
  (if (Variables|Default|GetIsBoosting)
    (Variables|Default|SetFuel (- (Variables|Default|GetFuel) (* (Variables|Default|GetFuelConsumption) DeltaTime (* (Variables|Default|GetBoostCostMultiplier) (Variables|/Game/KartVehicle/BP_Kart.BP_Kart_C|GetSpeedModifer (.AsBP%20Kart (Utilities|Casting|CastToBP_Kart (Game|Player|GetPlayerPawn 0))))) (Math|Float|Absolute(Float) (Variables|/Game/KartVehicle/BP_Kart.BP_Kart_C|GetAccelerationInput _returnvalue)))))
    (else
      (Variables|Default|SetFuel (- (Variables|Default|GetFuel) (* (Variables|Default|GetFuelConsumption) DeltaTime (Math|Float|Absolute(Float) (Variables|/Game/KartVehicle/BP_Kart.BP_Kart_C|GetAccelerationInput _returnvalue))))))))

(event Custom|Timer
  (params (DeltaTime :type Float%20%28double-precision%29))
  (Variables|Default|SetTimeElapsed (+ DeltaTime (Variables|Default|GetTimeElapsed)))
  (Variables|Default|SetLapTime (+ DeltaTime (Variables|Default|GetLapTime))))

(event Custom|Set%20Best%20Lap%20Time
  (if (or (< (Variables|Default|GetLapTime) (Variables|Default|GetBestLapTime)) (== (Variables|Default|GetBestLapTime) 0.0))
    (Variables|Default|SetBestLapTime (Variables|Default|GetLapTime)))
  (Variables|Default|SetLapTime 0.0))

(event Custom|FinalizeRace
  (Variables|Default|SetIsRaceFinished true)
  (CallFunction|SetBestLapTime)
  (Development|PrintText (Utilities|Text|FormatText "Final Time: {Time Elapsed} 
Best Lap Time: {Best Lap Time}" (Variables|Default|GetTimeElapsed) (Variables|Default|GetBestLapTime))))

(event EventBeginPlay)

(event EventTick
  (params (DeltaSeconds :type Float%20%28single-precision%29))
  (if (not (Variables|Default|GetIsRaceFinished))
    (if (> (Variables|Default|GetFuel) 0.0)
      (CallFunction|DecreaseFuel DeltaSeconds)
      (else
        (Variables|Default|SetFuel 0.0)))
    (CallFunction|Timer DeltaSeconds)))

(fn ConstructionScript)